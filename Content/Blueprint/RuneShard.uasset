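; Rune shard actor that hovers in the level and plays a sound when something overlaps its activation component.
; On BeginPlay it caches the static mesh's world location, then plays the RuneStoneHover timeline, whose vector track offsets the actor from that point.
; The RuneActivation overlap only triggers the sound at the mesh's location, with no pickup or state change.
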(event `self.ReceiveBeginPlay`
  ;[0 0 0] Initializes Rune Stones location as Vector
  (set `self.Initial Rune Location` (`SceneComponent.K2_GetComponentLocation` (`self.StaticMesh`)))
  ;[0 0 0] Automates the height of the Rune Stone so it moves up and down automaticaly
  (bind (_direction _movement_vector) (`Timeline|Rune Stone Hover`) ; Over 1.5seconds, adds a total of 150 to the Y vector
    (:`Update`
      (`self.K2_SetActorLocationAndRotation` (+ _movement_vector (`self.Initial Rune Location`))))))

(event `self.RuneActivation.OnComponentBeginOverlap`
  (params (OverlappedComponent :type "PrimitiveComponent Object Reference") (OtherActor :type "Actor Object Reference") (OtherComp :type "PrimitiveComponent Object Reference") (OtherBodyIndex :type Integer) (bFromSweep :type Boolean) (SweepResult :type "HitResult Structure (by ref)"))
  ;[0.1886 0 0.276] Sound
  (`GameplayStatics.PlaySoundAtLocation` null (`SceneComponent.K2_GetComponentLocation` (`self.StaticMesh`)) (struct) 1.0 1.0 0.0 null null null))

(fn `UserConstructionScript`)