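; Singing mushroom prop that randomizes its mesh and trigger box scale on construction and its material colors on BeginPlay.
; The first overlap by the ThirdPersonCharacter plays a random-pitched sound and shows a randomly colored point light.
; A timeline drives light intensity and the second dynamic material's brightness.
; Each finish replays it after a random delay with a globally attenuated sound, so the mushroom keeps singing and pulsing indefinitely.
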(event `self.ReceiveBeginPlay`
  (bind _staticmesh (`self.StaticMesh`))
  ;[1 1 1] Create Material Instances
  (`|ExecutionSequence`
    (:`then_0`
      (bind _returnvalue (`KismetMaterialLibrary.CreateDynamicMaterialInstance` "/Game/Material/Mushroom/MushroomGil.MushroomGil"))
      (`MaterialInstanceDynamic.SetVectorParameterValue` _returnvalue "Color" (make `LinearColor` (`KismetMathLibrary.RandomFloatInRange` 0.0 0.5) (`KismetMathLibrary.RandomFloatInRange` 0.0 0.5) (`KismetMathLibrary.RandomFloatInRange` 0.0 0.5) 1.0))
      (`PrimitiveComponent.SetMaterial` (`self.StaticMesh`) 0 _returnvalue))
    (:`then_1`
      (bind _returnvalue_2 (`KismetMaterialLibrary.CreateDynamicMaterialInstance` "/Game/Material/Mushroom/Material_Instances/MushroomGil_Inst.MushroomGil_Inst"))
      (`MaterialInstanceDynamic.SetVectorParameterValue` _returnvalue_2 "Color" (make `LinearColor` (`KismetMathLibrary.RandomFloatInRange` 0.0 0.5) (`KismetMathLibrary.RandomFloatInRange` 0.0 0.5) (`KismetMathLibrary.RandomFloatInRange` 0.0 0.5) 1.0))
      (`PrimitiveComponent.SetMaterial` _staticmesh 1 _returnvalue_2)
      (`PrimitiveComponent.SetMaterial` _staticmesh 2 _returnvalue_2))))

(event `self.ReceiveTick`
  (params (DeltaSeconds :type "Float (single-precision)")))

(event `self.Box.OnComponentBeginOverlap`
  (params (OverlappedComponent :type "PrimitiveComponent Object Reference") (OtherActor :type "Actor Object Reference") (OtherComp :type "PrimitiveComponent Object Reference") (OtherBodyIndex :type Integer) (bFromSweep :type Boolean) (SweepResult :type "HitResult Structure (by ref)"))
  (bind _pointlight (`self.PointLight`))
  ;[1 1 1] Change Color of Light and material
  (`/Engine/EditorBlueprintResources/StandardMacros.DoOnce` false
    (:`Completed`
      (cast `/Game/ThirdPersonBP/Blueprints/ThirdPersonCharacter` OtherActor)
      (`GameplayStatics.PlaySoundAtLocation` "/Game/Sound/Mushroom_Activation.Mushroom_Activation" (`SceneComponent.K2_GetComponentLocation` (`self.StaticMesh`)) (struct) 1.0 (`KismetMathLibrary.RandomFloatInRange` 0.125 0.5) 0.0 "/Game/Sound/Local_Sound.Local_Sound" null null)
      (`LightComponent.SetLightColor` _pointlight (`KismetMathLibrary.Conv_ColorToLinearColor` (`KismetMathLibrary.Conv_LinearColorToColor` (make `LinearColor` (`KismetMathLibrary.RandomFloatInRange` 0.0 0.5) (`KismetMathLibrary.RandomFloatInRange` 0.0 0.5) (`KismetMathLibrary.RandomFloatInRange` 0.0 0.5) 1.0))) true)
      (`SceneComponent.SetVisibility` _pointlight true false)
      (bind (_direction _newtrack_0) (`Timeline|Timeline_0` :!via `PlayFromStart` :!label _label)
        (:`Update`
          (`MaterialInstanceDynamic.SetScalarParameterValue` (stale `self.ReceiveBeginPlay` _returnvalue_2) "Brightness" _newtrack_0)
          (`LightComponent.SetIntensity` (`self.PointLight`) (* _newtrack_0 200000.0)))
        (:`Finished`
          ;[1 1 1] Play a looping sound
          (`KismetSystemLibrary.Delay` (`KismetMathLibrary.RandomFloatInRange` 2.0 5.0))
          (`GameplayStatics.PlaySoundAtLocation` "/Game/Sound/Mushroom_Activation.Mushroom_Activation" (`SceneComponent.K2_GetComponentLocation` (`self.StaticMesh`)) (struct) 1.0 (`KismetMathLibrary.RandomFloatInRange` 0.125 0.5) 0.0 "/Game/Sound/Global_sound.Global_sound" null null)
          (goto _label :!via `PlayFromStart`))))))

(fn `UserConstructionScript`
  (bind _returnvalue (`KismetMathLibrary.RandomFloatInRange` 1.0 5.0))
  (bind _returnvalue_2 (`KismetMathLibrary.RandomFloatInRange` 0.5 5.0))
  (bind _returnvalue_3 (* _returnvalue 11.5))
  (`SceneComponent.SetWorldScale3D` (`self.StaticMesh`) (`KismetMathLibrary.MakeVector` _returnvalue_2 _returnvalue_2 _returnvalue))
  (`SceneComponent.SetWorldScale3D` (`self.Box`) (`KismetMathLibrary.MakeVector` _returnvalue_3 _returnvalue_3 _returnvalue_3)))