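; Pushable rock prop that randomizes its look and gets shoved when the player character hits it.
; The construction script picks one of five rock meshes and scales each axis randomly; a roll of 5 has no case, leaving mesh and scale unchanged.
; On a hit by player character 0, the static mesh receives a large mass-dependent impulse along that character's forward vector.
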(event `self.ReceiveHit`
  (params (MyComp :type "PrimitiveComponent Object Reference") (Other :type "Actor Object Reference") (OtherComp :type "PrimitiveComponent Object Reference") (bSelfMoved :type Boolean) (HitLocation :type "Vector Structure") (HitNormal :type "Vector Structure") (NormalImpulse :type "Vector Structure") (Hit :type "HitResult Structure (by ref)"))
  (bind _returnvalue (`GameplayStatics.GetPlayerCharacter` 0))
  (if (== Other _returnvalue)
    (`PrimitiveComponent.AddImpulse` (`self.StaticMeshComponent`) (* (`self.GetActorForwardVector` _returnvalue) 100000.0) "None" false)))

(fn `UserConstructionScript`
  (bind _returnvalue (`KismetMathLibrary.RandomFloatInRange` 0.5 2.0))
  (bind _staticmeshcomponent (`self.StaticMeshComponent`))
  (switch `int` (`KismetMathLibrary.RandomIntegerInRange` 0 5)
    (:`0`
      (`StaticMeshComponent.SetStaticMesh` _staticmeshcomponent "/Game/Models/Rocks/medium/M_Rock1.M_Rock1"))
    (:`1`
      (`StaticMeshComponent.SetStaticMesh` _staticmeshcomponent "/Game/Models/Rocks/medium/M_Rock2.M_Rock2"))
    (:`2`
      (`StaticMeshComponent.SetStaticMesh` _staticmeshcomponent "/Game/Models/Rocks/medium/M_Rock3.M_Rock3"))
    (:`3`
      (`StaticMeshComponent.SetStaticMesh` _staticmeshcomponent "/Game/Models/Rocks/medium/M_Rock4.M_Rock4"))
    (:`4`
      (`StaticMeshComponent.SetStaticMesh` _staticmeshcomponent "/Game/Models/Rocks/medium/M_Rock5.M_Rock5")))
  (`SceneComponent.SetWorldScale3D` (`self.StaticMeshComponent`) (`KismetMathLibrary.MakeVector` _returnvalue _returnvalue _returnvalue)))